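; A test laser weapon Blueprint whose only working logic is material setup in the construction script.
; After the parent construction script runs, it applies OverrideMaterial to material slot 1 of every static and skeletal mesh component.
; BeginPlay and Tick are empty.
; An unconnected, never-executed draft would debug-draw a Visibility line trace from the muzzle along the first-person camera's forward vector.
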(event EventBeginPlay)

(event Collision|EventActorBeginOverlap
  (params (OtherActor :type Actor%20Object%20Reference)))

(event EventTick
  (params (DeltaSeconds :type Float%20%28single-precision%29)))

(fn ConstructionScript
  (|CallParentFunction)
  (for _array_element (Actor|GetComponentsByClass "/Script/Engine.StaticMeshComponent")
    (Rendering|Material|SetMaterial _array_element 1 (Variables|Default|GetOverrideMaterial)))
  (for _array_element_2 (Actor|GetComponentsByClass "/Script/Engine.SkeletalMeshComponent")
    (Rendering|Material|SetMaterial _array_element_2 1 (Variables|Default|GetOverrideMaterial))))