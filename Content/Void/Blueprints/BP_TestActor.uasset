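; BP_TestActor is a test actor that oscillates back and forth along the world X axis from where it starts.
; BeginPlay stores the start location, and a timeline's XPos track is added to its X on each update, with Y and Z held at their start values.
; Tick starts the timeline whenever it is idle, and its Finished event flips playback direction to create a continuous ping-pong.
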(event EventBeginPlay
  (Variables|Default|SetStartLocation (Transformation|GetActorLocation)))

(event EventTick
  (params (DeltaSeconds :type Float%20%28single-precision%29))
  (bind _startlocation (Variables|Default|GetStartLocation))
  (if (not (Audio|Components|Audio|IsPlaying (Variables|Default|GetTimeline)))
    (bind (_direction _x_pos) (Timeline|Timeline Play)
      (:Update
        (Transformation|SetActorLocation (Math|Vector|MakeVector (+ _x_pos (.x _startlocation)) (.y _startlocation) (.z _startlocation)) false false))
      (:Finished
        (switch Utilities|FlowControl|Switch|SwitchonETimelineDirection _direction
          (:Forward
            (Timeline|Timeline ReverseFromEnd))
          (:Backward
            (Timeline|Timeline PlayFromStart)))))))

(fn ConstructionScript)